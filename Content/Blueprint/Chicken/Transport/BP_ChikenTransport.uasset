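; BP_ChikenTransport is a chicken transporter character that holds the state for a transport job.
; On BeginPlay it casts the player controller to BPC_Rahoul and stores the reference.
; Getter and setter functions expose the transport value and the storage and resource references, with speed applied directly to CharacterMovement's MaxWalkSpeed.
; It contains no movement or hauling logic of its own.
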(event `self.ReceiveBeginPlay`
  (bind _asbpc_rahoul (cast `/Game/Blueprint/Rahoul/BPC_Rahoul` (`GameplayStatics.GetPlayerController` 0)))
  (set `self.RefPlayerController` _asbpc_rahoul))

(fn `GetRefRessource`
  (returns (RefRessource :type "/Game/Blueprint/Ressources/Bp_Ressources Object Reference"))
  (return (`self.RefRessource`)))

(fn `GetRefStorage`
  (returns (RefStorage :type "/Game/Blueprint/Ressources/Bp_storage Object Reference"))
  (return (`self.RefStorage`)))

(fn `GetSpeed`
  (returns (`Max Walk Speed` :type "Float (single-precision)"))
  (return (`CharacterMovementComponent.MaxWalkSpeed` (`self.CharacterMovement`))))

(fn `GetTransport`
  (returns (TransportUpdate :type Integer))
  (return (`self.TransportUpdate`)))

(fn `SetRefRessource`
  (params (RefRessource :type "/Game/Blueprint/Ressources/Bp_Ressources Object Reference"))
  (set `self.RefRessource` RefRessource))

(fn `SetRefStorage`
  (params (RefStorage :type "/Game/Blueprint/Ressources/Bp_storage Object Reference"))
  (set `self.RefStorage` RefStorage))

(fn `setSpeed`
  (params (Speedmodif :type "Float (double-precision)"))
  (bind _output_get (set `self.Speedmodif` Speedmodif))
  (set `CharacterMovementComponent.MaxWalkSpeed` _output_get (`self.CharacterMovement`)))

(fn `setTransport`
  (params (TransportUpdate :type Integer))
  (set `self.TransportUpdate` TransportUpdate))

(fn `UserConstructionScript`)