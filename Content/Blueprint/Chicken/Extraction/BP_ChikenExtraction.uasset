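; BP_ChikenExtraction is an extraction tool actor that displays either a pickaxe or an axe with a looping animation.
; Shortly after BeginPlay, the ETypeExtractor value selects the mesh for StaticMesh1.
; In parallel, a Timeline drives the actor's roll and the StaticMesh component's relative Y offset.
; The Timeline replays from the start each time it finishes, through a restart event.
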(event `self.ReceiveBeginPlay`
  (bind (_returnvalue_roll _returnvalue_pitch _returnvalue_yaw) (`KismetMathLibrary.BreakRotator` (`self.K2_GetActorRotation`)))
  (bind _staticmesh1 (`self.StaticMesh1`))
  (`|ExecutionSequence`
    (:`then_0`
      (`KismetSystemLibrary.Delay` 0.2)
      (switch `/Game/Blueprint/Chicken/Extraction/E_TypeExtractor` (`self.ETypeExtractor`)
        (:`NewEnumerator0`
          (`StaticMeshComponent.SetStaticMesh` _staticmesh1 "/Game/Assets/Pickaxe/Pickaxe_pCube3.Pickaxe_pCube3"))
        (:`NewEnumerator1`
          (`StaticMeshComponent.SetStaticMesh` _staticmesh1 "/Game/Asset/Axe/SM_Axe.SM_Axe"))))
    (:`then_1`
      (bind (_direction _newtrack_0) (`Timeline|Timeline` :!via `PlayFromStart` :!label _label)
        (:`Update`
          (`self.K2_SetActorRotation` (`KismetMathLibrary.MakeRotator` (* 10.0 _newtrack_0) _returnvalue_pitch _returnvalue_yaw))
          (`SceneComponent.K2_SetRelativeLocation` (`self.StaticMesh`) (`KismetMathLibrary.MakeVector` 0.0 (* 10.0 _newtrack_0)) false false))
        (:`Finished`
          (`self.restart`))))))

(event `restart`
  (goto _label :!via `PlayFromStart`))

(fn `UserConstructionScript`)