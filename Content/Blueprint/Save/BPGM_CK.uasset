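; BPGM_CK manages the game's persistent save in the GlobalSave slot.
; Init loads the existing BP_Save from that slot or creates a new one, stores it as PlayerSave, then starts a looping one-minute timer.
; The SaveGame event writes the object returned by a SaveGame call back to the same slot.
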(event `self.ReceiveInit`
  (bind _returnvalue (`GameplayStatics.DoesSaveGameExist` "GlobalSave"))
  (if _returnvalue
    (bind _returnvalue_2 (`GameplayStatics.LoadGameFromSlot` "GlobalSave"))
    (bind _asbp_save (cast `/Game/Blueprint/Save/BP_Save` _returnvalue_2))
    (set `self.PlayerSave` _asbp_save)
    (else
      (bind _returnvalue_3 (`GameplayStatics.CreateSaveGameObject` "/Game/Blueprint/Save/BP_Save.BP_Save_C"))
      (set `self.PlayerSave` _returnvalue_3)))
  (`KismetSystemLibrary.K2_SetTimerDelegate` (`|CreateDelegate` :!event `SaveGame`) 60.0 true))

(event `SaveGame`
  (bind _savelocalref1 (`/Game/Blueprint/Save/BPFL_Save.SaveGame`))
  (`GameplayStatics.SaveGameToSlot` _savelocalref1 "GlobalSave"))