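; Blueprint function library for saving player data: resources, refined resources and chicken count.
; SaveGame fetches PlayerSave from the BPGM_CK game instance, runs three grouped steps in sequence, then returns that save object.
; Each step assigns the save object's fields back to themselves, so no values change and nothing is written to a save slot here.
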(fn `SaveGame`
  (returns (SaveLocalRef1 :type "/Game/Blueprint/Save/BP_Save Object Reference"))
  (locals (SaveLocalRef :type "/Game/Blueprint/Save/BP_Save Object Reference"))
  (bind _savelocalref (`local.SaveLocalRef`))
  (bind _savelocalref_2 (`local.SaveLocalRef`))
  (bind _savelocalref_3 (`local.SaveLocalRef`))
  (bind _savelocalref_4 (`local.SaveLocalRef`))
  (bind _savelocalref_5 (`local.SaveLocalRef`))
  (bind _savelocalref_6 (`local.SaveLocalRef`))
  (bind _savelocalref_7 (`local.SaveLocalRef`))
  (set `local.SaveLocalRef` (`/Game/Blueprint/Save/BPGM_CK.PlayerSave` (cast `/Game/Blueprint/Save/BPGM_CK` (`GameplayStatics.GetGameInstance` null) :!pure true)))
  (`|ExecutionSequence`
    (:`then_0`
      (set `/Game/Blueprint/Save/BP_Save.WoodAmount` (`/Game/Blueprint/Save/BP_Save.WoodAmount` _savelocalref) _savelocalref)
      (set `/Game/Blueprint/Save/BP_Save.StoneAmount` (`/Game/Blueprint/Save/BP_Save.StoneAmount` _savelocalref_2) _savelocalref_2)
      (set `/Game/Blueprint/Save/BP_Save.IronAmount` (`/Game/Blueprint/Save/BP_Save.IronAmount` _savelocalref_3) _savelocalref_3))
    (:`then_1`
      (set `/Game/Blueprint/Save/BP_Save.PlanksAmount` (`/Game/Blueprint/Save/BP_Save.PlanksAmount` _savelocalref_5) _savelocalref_5)
      (set `/Game/Blueprint/Save/BP_Save.BricksAmount` (`/Game/Blueprint/Save/BP_Save.BricksAmount` _savelocalref_6) _savelocalref_6)
      (set `/Game/Blueprint/Save/BP_Save.IronIngotAmount` (`/Game/Blueprint/Save/BP_Save.IronIngotAmount` _savelocalref_4) _savelocalref_4))
    (:`then_2`
      (set `/Game/Blueprint/Save/BP_Save.NumberOfChicken` (`/Game/Blueprint/Save/BP_Save.NumberOfChicken` _savelocalref_7) _savelocalref_7))
    (:`then_3`
      (return (`local.SaveLocalRef`)))))