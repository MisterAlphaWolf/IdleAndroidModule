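; Behavior tree service that deposits a chicken's carried resources into storage and points it back to its resource.
; When the service deactivates, it adds the chicken's carried amount to the wood, iron or stone count of the Bp_storage in the target blackboard key, based on its resource type.
; It then writes the chicken's resource reference to the new-target key and resets the carried amount to zero.
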(event `self.ReceiveDeactivationAI`
  (params (OwnerController :type "AIController Object Reference") (ControlledPawn :type "Pawn Object Reference"))
  (bind _asbp_storage (cast `/Game/Blueprint/Ressources/Bp_storage` (`BTFunctionLibrary.GetBlackboardValueAsObject` (`self.Key_Target`)) :!pure true))
  (bind _asbp_chiken (cast `/Game/Blueprint/AI/BP_Chiken` ControlledPawn))
  (switch `/Game/Blueprint/Ressources/ETypeRessources` (`/Game/Blueprint/AI/BP_Chiken.ETypeRessources` _asbp_chiken)
    (:`NewEnumerator0`
      (bind _nressources (`/Game/Blueprint/AI/BP_Chiken.NRessources` _asbp_chiken))
      (set `/Game/Blueprint/Ressources/Bp_storage.NWood` (+ _nressources (`/Game/Blueprint/Ressources/Bp_storage.NWood` _asbp_storage)) _asbp_storage))
    (:`NewEnumerator1`
      (set `/Game/Blueprint/Ressources/Bp_storage.NIron` (+ _nressources (`/Game/Blueprint/Ressources/Bp_storage.NIron` _asbp_storage)) _asbp_storage))
    (:`NewEnumerator2`
      (set `/Game/Blueprint/Ressources/Bp_storage.NStone` (+ _nressources (`/Game/Blueprint/Ressources/Bp_storage.NStone` _asbp_storage)) _asbp_storage)))
  (`BTFunctionLibrary.SetBlackboardValueAsObject` (`self.Key_NewTarget`) (`/Game/Blueprint/AI/BP_Chiken.RefRessource` _asbp_chiken))
  (set `/Game/Blueprint/AI/BP_Chiken.NRessources` 0 _asbp_chiken))