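; Behavior tree service that hands a chicken the contents of a resource target and redirects it to its storage.
; On deactivation, if the KeyTarget blackboard object is a resource, it copies that resource's type and amount onto the controlled BP_Chiken and zeroes the resource's amount.
; It then writes the chicken's RefStorage into the KeyNewTarget blackboard key.
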(event `self.ReceiveDeactivationAI`
  (params (OwnerController :type "AIController Object Reference") (ControlledPawn :type "Pawn Object Reference"))
  (bind (_asbp_ressources _bsuccess) (cast `/Game/Blueprint/Ressources/Bp_Ressources` (`BTFunctionLibrary.GetBlackboardValueAsObject` (`self.Key_Target`)) :!pure true))
  (if _bsuccess
    (bind _asbp_chiken (cast `/Game/Blueprint/AI/BP_Chiken` ControlledPawn))
    (set `/Game/Blueprint/AI/BP_Chiken.ETypeRessources` (`/Game/Blueprint/Ressources/Bp_Ressources.ETypeRessources` _asbp_ressources) _asbp_chiken)
    (set `/Game/Blueprint/AI/BP_Chiken.NRessources` (`/Game/Blueprint/Ressources/Bp_Ressources.NRessource` _asbp_ressources) _asbp_chiken)
    (set `/Game/Blueprint/Ressources/Bp_Ressources.NRessource` 0 _asbp_ressources)
    (`BTFunctionLibrary.SetBlackboardValueAsObject` (`self.Key_NewTarget`) (`/Game/Blueprint/AI/BP_Chiken.RefStorage` _asbp_chiken))))