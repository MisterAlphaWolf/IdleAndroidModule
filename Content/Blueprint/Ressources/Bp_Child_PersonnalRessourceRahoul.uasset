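; Child resource Blueprint that serves as a personal gathering zone for the BP_Rahoul character.
; Entering its Box stores a reference to Rahoul and starts a looping timer, which is cleared when Rahoul leaves.
; The RecupRahoul event is the harvest step, making several random draws that each add one wood, stone or iron directly to Rahoul's counters.
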(event `self.Box.OnComponentBeginOverlap`
  (params (OverlappedComponent :type "PrimitiveComponent Object Reference") (OtherActor :type "Actor Object Reference") (OtherComp :type "PrimitiveComponent Object Reference") (OtherBodyIndex :type Integer) (bFromSweep :type Boolean) (SweepResult :type "HitResult Structure (by ref)"))
  (bind _asbp_rahoul (cast `/Game/Blueprint/Rahoul/BP_Rahoul` OtherActor))
  (set `self.RefBPRahoul` _asbp_rahoul)
  (bind _returnvalue (`KismetSystemLibrary.K2_SetTimerDelegate` :`Time` 10.0 :`bLooping` true))
  (set `self.RefTimer` _returnvalue))

(event `self.Box.OnComponentEndOverlap`
  (params (OverlappedComponent :type "PrimitiveComponent Object Reference") (OtherActor :type "Actor Object Reference") (OtherComp :type "PrimitiveComponent Object Reference") (OtherBodyIndex :type Integer))
  (cast `/Game/Blueprint/Rahoul/BP_Rahoul` OtherActor)
  (`KismetSystemLibrary.K2_ClearAndInvalidateTimerHandle` (`self.RefTimer`)))

(event `RecupRahoul`
  (bind _refbprahoul (`self.RefBPRahoul`))
  (bind _refbprahoul_2 (`self.RefBPRahoul`))
  (bind _refbprahoul_3 (`self.RefBPRahoul`))
  (for _ (range 3)
    (switch `int` (`KismetMathLibrary.RandomIntegerInRange` 0 2)
      (:`0`
        (set `/Game/Blueprint/Rahoul/BP_Rahoul.WoodAmond` (+ 1 (`/Game/Blueprint/Rahoul/BP_Rahoul.WoodAmond` _refbprahoul)) _refbprahoul))
      (:`1`
        (set `/Game/Blueprint/Rahoul/BP_Rahoul.StoneAmond` (+ 1 (`/Game/Blueprint/Rahoul/BP_Rahoul.StoneAmond` _refbprahoul_2)) _refbprahoul_2))
      (:`2`
        (set `/Game/Blueprint/Rahoul/BP_Rahoul.IronAmond` (+ 1 (`/Game/Blueprint/Rahoul/BP_Rahoul.IronAmond` _refbprahoul_3)) _refbprahoul_3)))))

(fn `UserConstructionScript`
  (`parent.UserConstructionScript`))