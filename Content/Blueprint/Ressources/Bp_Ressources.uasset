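; Resource node actor (wood, iron or stone, which sets its mesh) that accumulates resources from the chicken extractors assigned to it.
; RessourceProduct starts at BeginPlay, adds the spawned count to the total and re-arms a one-second timer.
; It steps that count toward the assigned number, spawning extractors on random box edges, facing the node.
; Past ten, it recolors existing chickens by modulo index, advancing a color tier every ten.
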(event `self.ReceiveBeginPlay`
  (`self.RessourceProduct`))

(event `RessourceProduct`
  (bind _nspawnchiken_extract (`self.NSpawnChiken Extract`))
  (bind _refchickenextractor (`self.RefChickenExtractor`))
  (if (!= (`self.NChikenExtracte`) 0)
    (set `self.NRessource` (+ (`self.NRessource`) (`self.NSpawnChiken Extract`)))
    (if (> (`self.NChikenExtracte`) (`self.NSpawnChiken Extract`))
      (if (and (!= (`self.NSpawnChiken Extract`) 0) (> (`self.NSpawnChiken Extract`) 9))
        (if (not (!= (mod (`self.NSpawnChiken Extract`) 10) 0))
          (`/Engine/EditorBlueprintResources/StandardMacros.IncrementInt` (`self.LevelColor`)
            (:`  `
              _)))
        (`/Engine/EditorBlueprintResources/StandardMacros.IncrementInt` _nspawnchiken_extract
          (:`  `
            (`MeshComponent.SetVectorParameterValueOnMaterials` (`/Game/Blueprint/Chicken/Extraction/BP_ChikenExtraction.StaticMesh` (`|GetArrayItem` (`self.RefChickenExtractor`) (mod _nspawnchiken_extract 10))) "ColorChicken" (`|GetArrayItem` (`self.Parameter Value`) (`self.LevelColor`)))
            (`KismetSystemLibrary.PrintString` "changecolor")
            (`KismetSystemLibrary.K2_SetTimerDelegate` (`|CreateDelegate` :!event `RessourceProduct`) 1.0)))
        (else
          (bind _returnvalue (`self.SpawnChickenExtractor`))
          (bind _returnvalue_2 (`KismetArrayLibrary.Array_Add` _refchickenextractor _returnvalue))
          (`KismetSystemLibrary.PrintString` (`KismetSystemLibrary.GetDisplayName` (`|GetArrayItem` _refchickenextractor _returnvalue_2)) true true (struct :`R` 1.0 :`G` 0.674199 :`A` 1.0))
          (set `/Game/Blueprint/Chicken/Extraction/BP_ChikenExtraction.ETypeExtractor` (select `/Game/Blueprint/Ressources/ETypeRessources` (`self.ETypeRessources`) :`NewEnumerator0` "NewEnumerator1" :`NewEnumerator1` "NewEnumerator0" :`NewEnumerator2` "NewEnumerator0" :!type "/Game/Blueprint/Chicken/Extraction/E_TypeExtractor Enum") _returnvalue)
          (`/Engine/EditorBlueprintResources/StandardMacros.IncrementInt` (`self.NSpawnChiken Extract`)
            (:`  `
              (`self.K2_SetActorRotation` _returnvalue (`KismetMathLibrary.FindLookAtRotation` (`self.K2_GetActorLocation` _returnvalue) (`self.K2_GetActorLocation`)) false)
              (`KismetSystemLibrary.K2_SetTimerDelegate` (`|CreateDelegate` :!event `RessourceProduct`) 1.0)))))
      (else
        (`KismetSystemLibrary.K2_SetTimerDelegate` (`|CreateDelegate` :!event `RessourceProduct`) 1.0)))
    (else
      (`KismetSystemLibrary.K2_SetTimerDelegate` (`|CreateDelegate` :!event `RessourceProduct`) 1.0))))

(event `addChickenExtractor`
  (`/Engine/EditorBlueprintResources/StandardMacros.IncrementInt` (`self.NChikenExtracte`)))

(fn `GetNchickenExtractor`
  (returns (NChikenExtracte :type Integer))
  (return (`self.NChikenExtracte`)))

(fn `SetNchickenExtractor`
  (params (NChikenExtracte :type Integer))
  (set `self.NChikenExtracte` NChikenExtracte))

(fn `SpawnChickenExtractor`
  (returns (ReturnValue :type "/Game/Blueprint/Chicken/Extraction/BP_ChikenExtraction Object Reference"))
  (bind (_origin _boxextent) (`KismetSystemLibrary.GetComponentBounds` (`self.Box`)))
  (bind _returnvalue (* (.y _boxextent) -1.0))
  (bind _returnvalue_2 (* (.x _boxextent) -1.0))
  (set `self.ExternBounds` (select `bool` (`KismetMathLibrary.RandomBool`) :`false` (`KismetMathLibrary.MakeVector` (select `bool` (`KismetMathLibrary.RandomBool`) :`false` (.x _boxextent) :`true` _returnvalue_2) (`KismetMathLibrary.RandomFloatInRange` _returnvalue (.y _boxextent))) :`true` (`KismetMathLibrary.MakeVector` (`KismetMathLibrary.RandomFloatInRange` _returnvalue_2 (.x _boxextent)) (select `bool` (`KismetMathLibrary.RandomBool`) :`false` (.y _boxextent) :`true` _returnvalue)) :!type "Vector Structure"))
  (bind _returnvalue_3 (`|SpawnActorFromClass` "/Game/Blueprint/Chicken/Extraction/BP_ChikenExtraction.BP_ChikenExtraction_C" (`KismetMathLibrary.MakeTransform` (+ (`self.K2_GetActorLocation`) (`self.ExternBounds`))) "AdjustIfPossibleButAlwaysSpawn" "MultiplyWithRoot" null null))
  (return _returnvalue_3))

(fn `UserConstructionScript`
  (switch `/Game/Blueprint/Ressources/ETypeRessources` (`self.ETypeRessources`)
    (:`NewEnumerator0`
      (`StaticMeshComponent.SetStaticMesh` (`self.RessourceMesh`) "/Game/Assets/City_Kit_Suburban/FBX_format/Trees/detail_treeLarge_detail_treeLarge.detail_treeLarge_detail_treeLarge"))
    (:`NewEnumerator1`
      (`StaticMeshComponent.SetStaticMesh` (`self.RessourceMesh`) "/Game/Assets/Space/Models/FBX_format/Rocks/rock_crystalsLargeA_rock_crystalsLargeA.rock_crystalsLargeA_rock_crystalsLargeA"))
    (:`NewEnumerator2`
      (`StaticMeshComponent.SetStaticMesh` (`self.RessourceMesh`) "/Game/Assets/Space/Models/FBX_format/Rocks/rock_largeA_rock_largeA.rock_largeA_rock_largeA"))))