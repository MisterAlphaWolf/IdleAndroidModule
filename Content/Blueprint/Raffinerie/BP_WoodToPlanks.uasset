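; Refinery actor that converts the player's wood into planks on a timer, with a floating resource mesh as visual feedback.
; On BeginPlay it caches the BPC_Rahoul player controller and starts a looping timer, apparently driving AddPlanksToInventory, which sets Planks to the Wood value without deducting wood.
; Two chained timelines bob the resource via VInterpTo, repeating until EnoughtRessource is set.
; Debug prints show the timer's remaining time.
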(event `AddPlanksToInventory`
  (`KismetSystemLibrary.PrintString` "Hello")
  (`/Game/Blueprint/Rahoul/BPC_Rahoul.SetPlanks` (`self.BPC_Rahoul_Ref`) (`/Game/Blueprint/Rahoul/BPC_Rahoul.GetWood` (`self.BPC_Rahoul_Ref`))))

(event `self.ReceiveTick`
  (params (DeltaSeconds :type "Float (single-precision)"))
  (`KismetSystemLibrary.PrintString` (`KismetStringLibrary.Conv_DoubleToString` (`KismetSystemLibrary.K2_GetTimerRemainingTimeHandle` (stale `ConvertingWoodToPlanks` _returnvalue))) true true (struct :`G` 0.66 :`B` 1.0 :`A` 1.0) 0.0))

(event `ConvertingWoodToPlanks`
  (bind _returnvalue (`KismetSystemLibrary.K2_SetTimerDelegate` (`|CreateDelegate` :!event `AddPlanksToInventory`) 5.0 true)))

(event `self.ReceiveBeginPlay`
  (`self.FloatRessource`)
  (bind _asbpc_rahoul (cast `/Game/Blueprint/Rahoul/BPC_Rahoul` (`GameplayStatics.GetPlayerController` 0)))
  (set `self.BPC_Rahoul_Ref` _asbpc_rahoul)
  (`self.ConvertingWoodToPlanks`))

(event `FloatRessource`
  (bind _returnvalue (`SceneComponent.K2_GetComponentLocation` (`self.Ressource`)))
  (bind _returnvalue_2 (`SceneComponent.K2_GetComponentLocation` (`self.Ressource`)))
  (bind (_direction _float) (`Timeline|RessourceFloat` :!via `PlayFromStart`)
    (:`Update`
      (`SceneComponent.K2_SetWorldLocation` (`self.Ressource`) (`KismetMathLibrary.VInterpTo` _returnvalue_2 (`KismetMathLibrary.MakeVector` (.x _returnvalue_2) (.y _returnvalue_2) (+ (.z _returnvalue_2) _float)) (`GameplayStatics.GetWorldDeltaSeconds`) 200.0) false false))
    (:`Finished`
      (bind (_direction_2 _float_2) (`Timeline|RessourceFloat2` :!via `PlayFromStart`)
        (:`Update`
          (`SceneComponent.K2_SetWorldLocation` (`self.Ressource`) (`KismetMathLibrary.VInterpTo` _returnvalue (`KismetMathLibrary.MakeVector` (.x _returnvalue) (.y _returnvalue) (+ (.z _returnvalue) _float_2)) (`GameplayStatics.GetWorldDeltaSeconds`) 200.0) false false))
        (:`Finished`
          (if (not (`self.EnoughtRessource`))
            (`self.FloatRessource`)))))))

(fn `UserConstructionScript`)