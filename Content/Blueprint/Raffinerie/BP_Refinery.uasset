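; Refinery building that turns the wood, stone or iron selected by ChangeRessources into planks, bricks or iron ingots for the player.
; Construction script picks the matching resource mesh; activation starts effects, a looping two-timeline float animation and a loading widget.
; A looping timer is started for conversion, while AddRessourcesToInventory decrements storage, increments the player controller's count and refreshes the HUD.
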(event `AddRessourcesToInventory`
  (bind _bpc_rahoul_ref (`self.BPC_Rahoul_Ref`))
  (bind _refbp_storage (`self.RefBP_Storage`))
  (bind _refbp_storage_2 (`self.RefBP_Storage`))
  (bind _refbp_storage_3 (`self.RefBP_Storage`))
  (bind _bpc_rahoul_ref_2 (`self.BPC_Rahoul_Ref`))
  (bind _bpc_rahoul_ref_3 (`self.BPC_Rahoul_Ref`))
  (switch `/Game/Blueprint/Raffinerie/Refinery_Ressources` (`self.Change_Ressources`)
    (:`NewEnumerator0`
      (`/Game/Blueprint/Rahoul/BPC_Rahoul.SetPlanks` _bpc_rahoul_ref (+ (`/Game/Blueprint/Rahoul/BPC_Rahoul.GetPlanks` _bpc_rahoul_ref) 1))
      (`/Game/Blueprint/Justine/WBP_HUD.SetTextPlank` (`/Game/Blueprint/Rahoul/BPC_Rahoul.HUD Ref` (`self.BPC_Rahoul_Ref`)))
      (`/Engine/EditorBlueprintResources/StandardMacros.DecrementInt` (`/Game/Blueprint/Ressources/Bp_storage.NWood` _refbp_storage_2)
        (:`  `
          (`/Game/Blueprint/Ressources/Bp_storage.UpdateWood` _refbp_storage_2))))
    (:`NewEnumerator1`
      (`/Game/Blueprint/Rahoul/BPC_Rahoul.SetBricks` _bpc_rahoul_ref_2 (+ (`/Game/Blueprint/Rahoul/BPC_Rahoul.GetBricks` _bpc_rahoul_ref_2) 1))
      (`/Game/Blueprint/Justine/WBP_HUD.SetTextBrick` (`/Game/Blueprint/Rahoul/BPC_Rahoul.HUD Ref` (`self.BPC_Rahoul_Ref`)))
      (`/Engine/EditorBlueprintResources/StandardMacros.DecrementInt` (`/Game/Blueprint/Ressources/Bp_storage.NStone` _refbp_storage_3)
        (:`  `
          (`/Game/Blueprint/Ressources/Bp_storage.UpdateStone` _refbp_storage_3))))
    (:`NewEnumerator2`
      (`/Game/Blueprint/Rahoul/BPC_Rahoul.SetIronIngot` _bpc_rahoul_ref_3 (+ (`/Game/Blueprint/Rahoul/BPC_Rahoul.GetIronIngot` _bpc_rahoul_ref_3) 1))
      (`/Game/Blueprint/Justine/WBP_HUD.SetTextIronIngot` (`/Game/Blueprint/Rahoul/BPC_Rahoul.HUD Ref` (`self.BPC_Rahoul_Ref`)))
      (`/Engine/EditorBlueprintResources/StandardMacros.DecrementInt` (`/Game/Blueprint/Ressources/Bp_storage.NIron` _refbp_storage)
        (:`  `
          (`/Game/Blueprint/Ressources/Bp_storage.UpdateIron` _refbp_storage))))))

(event `RaffinerieIsBuy`
  (`ActorComponent.K2_DestroyComponent` (`self.woodStructure_high_woodStructure_high`)))

(event `ConvertingRessources`
  (`self.DisplayWidget`)
  (`KismetSystemLibrary.K2_SetTimerDelegate` (`|CreateDelegate` :!event `AddRessourcesToInventory`) 10.0 true))

(event `DisplayWidget`
  (bind _returnvalue (`WidgetComponent.GetWidget` (`self.Widget`)))
  (bind _aswbp_loading (cast `/Game/Blueprint/Justine/WBP_Loading` _returnvalue :!pure true))
  (`Widget.SetVisibility` _returnvalue "Visible")
  (`/Game/Blueprint/Justine/WBP_Loading.SetRessourceIcon` _aswbp_loading (select `/Game/Blueprint/Raffinerie/Refinery_Ressources` (`self.Change_Ressources`) :`NewEnumerator0` "/Game/Asset/UI/Shikashi_s_Fantasy_Icons_Pack_v2/_1_-_Transparent_Icons_Sprite_306._1_-_Transparent_Icons_Sprite_306" :`NewEnumerator1` "/Game/Asset/UI/Brick.Brick" :`NewEnumerator2` "/Game/Asset/UI/IronIngot.IronIngot" :!type "Object Object Reference"))
  (`UserWidget.AddToViewport` _aswbp_loading 0))

(event `ActivateRaffinerie`
  (if (not (`self.RaffinerieBuy?`))
    (`self.RaffinerieActivate`)
    (`self.FloatRessource`)
    (bind _asbpc_rahoul (cast `/Game/Blueprint/Rahoul/BPC_Rahoul` (`GameplayStatics.GetPlayerController` 0)))
    (set `self.BPC_Rahoul_Ref` _asbpc_rahoul)
    (`self.ConvertingRessources`)))

(event `FloatRessource`
  (bind _returnvalue (`SceneComponent.K2_GetComponentLocation` (`self.Ressource`)))
  (bind _returnvalue_2 (`SceneComponent.K2_GetComponentLocation` (`self.Ressource`)))
  (bind (_direction _float) (`Timeline|RessourceFloat` :!via `PlayFromStart`)
    (:`Update`
      (`SceneComponent.K2_SetWorldLocation` (`self.Ressource`) (`KismetMathLibrary.VInterpTo` _returnvalue_2 (`KismetMathLibrary.MakeVector` (.x _returnvalue_2) (.y _returnvalue_2) (+ (.z _returnvalue_2) _float)) (`GameplayStatics.GetWorldDeltaSeconds`) 200.0) false false))
    (:`Finished`
      (bind (_direction_2 _float_2) (`Timeline|RessourceFloat2` :!via `PlayFromStart`)
        (:`Update`
          (`SceneComponent.K2_SetWorldLocation` (`self.Ressource`) (`KismetMathLibrary.VInterpTo` _returnvalue (`KismetMathLibrary.MakeVector` (.x _returnvalue) (.y _returnvalue) (+ (.z _returnvalue) _float_2)) (`GameplayStatics.GetWorldDeltaSeconds`) 200.0) false false))
        (:`Finished`
          (if (not (`self.EnoughtRessource`))
            (`self.FloatRessource`)))))))

(fn `RaffinerieActivate`
  (`ActorComponent.Activate` (`self.P_Smoke`) false)
  (`ActorComponent.Activate` (`self.P_Sparks`) false)
  (`ActorComponent.Activate` (`self.P_FireRafinerie`) false)
  (`SceneComponent.SetHiddenInGame` (`self.Ressource`) false false)
  (return))

(fn `UserConstructionScript`
  (switch `/Game/Blueprint/Raffinerie/Refinery_Ressources` (`self.Change_Ressources`)
    (:`NewEnumerator0`
      (`StaticMeshComponent.SetStaticMesh` (`self.Ressource`) "/Game/Assets/Nature/Models/FBX_format/Wood/log_stack.log_stack"))
    (:`NewEnumerator1`
      (`StaticMeshComponent.SetStaticMesh` (`self.Ressource`) "/Game/Assets/Space/Models/FBX_format/Rocks/rocks_smallA.rocks_smallA"))
    (:`NewEnumerator2`
      (`StaticMeshComponent.SetStaticMesh` (`self.Ressource`) "/Game/Assets/Tower_Defense/Models/FBX_format/Crystal/IronNeggets.IronNeggets"))))