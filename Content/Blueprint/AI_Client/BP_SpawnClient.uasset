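; Spawner actor that creates half-scale BP_Client actors and sends them walking between six Billboard reference points, with the first Billboard acting as a hub.
; A random index picks the start: clients from outer points move to the hub, while clients from the hub move to a random outer point, re-rolled through Reload.
; Each spawn then sets a one-shot timer with a random delay of a few seconds.
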(event `self.ReceiveBeginPlay`
  (set `self.RefPosition` (`|MakeArray` (`self.Billboard`) (`self.Billboard1`) (`self.Billboard2`) (`self.Billboard3`) (`self.Billboard4`) (`self.Billboard5`)))
  (`self.spawn`))

(event `spawn`
  (bind _output_get (set `self.ElementSpawnPosition` (`.OutIndex` (`KismetArrayLibrary.Array_Random` (`self.RefPosition`)))))
  (if (!= _output_get 0)
    (bind _returnvalue (`|SpawnActorFromClass` "/Game/Blueprint/AI_Client/BP_Client.BP_Client_C" (`KismetMathLibrary.MakeTransform` (`SceneComponent.K2_GetComponentLocation` (`|GetArrayItem` (`self.RefPosition`) (`self.ElementSpawnPosition`))) (struct) (0.5 0.5 0.5)) "AdjustIfPossibleButAlwaysSpawn" "MultiplyWithRoot" null null))
    (`KismetSystemLibrary.PrintString` (`KismetStringLibrary.Conv_VectorToString` (`self.K2_GetActorLocation` _returnvalue)))
    (`/Game/Blueprint/AI_Client/BP_Client.MoveTo` _returnvalue (`SceneComponent.K2_GetComponentLocation` (`self.Billboard`)))
    (`KismetSystemLibrary.K2_SetTimerDelegate` (`|CreateDelegate` :!event `spawn`) (`KismetMathLibrary.RandomFloatInRange` 1.0 5.0))
    (else
      (bind _output_get_2 (set `self.ElementEndPosition` (`.OutIndex` (`KismetArrayLibrary.Array_Random` (`self.RefPosition`))) :!label _label))
      (if (!= _output_get_2 0)
        (bind _returnvalue_2 (`|SpawnActorFromClass` "/Game/Blueprint/AI_Client/BP_Client.BP_Client_C" (`KismetMathLibrary.MakeTransform` (`SceneComponent.K2_GetComponentLocation` (`|GetArrayItem` (`self.RefPosition`) (`self.ElementSpawnPosition`))) (struct) (0.5 0.5 0.5)) "AdjustIfPossibleButAlwaysSpawn" "MultiplyWithRoot" null null))
        (`/Game/Blueprint/AI_Client/BP_Client.MoveTo` _returnvalue_2 (`SceneComponent.K2_GetComponentLocation` (`|GetArrayItem` (`self.RefPosition`) (`self.ElementEndPosition`))))
        (`KismetSystemLibrary.K2_SetTimerDelegate` (`|CreateDelegate` :!event `spawn`) (`KismetMathLibrary.RandomFloatInRange` 1.0 5.0))
        (else
          (`self.Reload`))))))

(event `Reload`
  (goto _label))

(fn `UserConstructionScript`)