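; Player controller for Rahoul that provides touch-to-move control of the possessed pawn through Enhanced Input.
; Starting a touch stops current movement, and holding it traces under the finger, caches the hit location and steers the pawn toward it with movement input.
; A press released or canceled within the time threshold sends the pawn to the cached location via SimpleMoveToLocation.
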(event `self.ReceiveBeginPlay`
  (bind _returnvalue (subsystem `EnhancedInputLocalPlayerSubsystem`))
  ;[1 1 1] Add Mapping Context
  (`/Engine/EditorBlueprintResources/StandardMacros.IsValid` _returnvalue
    (:`Is Valid`
      (`EnhancedInputSubsystemInterface.AddMappingContext` _returnvalue "/Game/Blueprint/Rahoul/Input/IMC_Movement.IMC_Movement" 0 (struct)))))

(event `EnhancedInput|/Game/Blueprint/Rahoul/Input/InputAction/IA_TouchToMove`
  (params (ActionValue :type Boolean) (ElapsedSeconds :type "Float (double-precision)") (TriggeredSeconds :type "Float (double-precision)") (InputAction :type "InputAction Object Reference" :default "/Game/Blueprint/Rahoul/Input/InputAction/IA_TouchToMove.IA_TouchToMove"))
  (bind (_hit _location) (`self.GetLocationUnderFinger`))
  (:`Triggered`
    (if _hit
      (bind _output_get (set `self.CachedLocation` _location))
      (`self.Follow` _output_get)))
  (:`Started`
    (`self.StopMovement`))
  (:`Canceled`
    (if (< ElapsedSeconds (`self.PressedThreshold`)) :!label _label
      (`self.MoveTo` (`self.CachedLocation`))))
  (:`Completed`
    (goto _label)))

(fn `Follow`
  (params (Location :type "Vector Structure"))
  (bind _returnvalue (`self.K2_GetPawn`))
  (`Pawn.AddMovementInput` _returnvalue (`KismetMathLibrary.GetDirectionUnitVector` (`self.K2_GetActorLocation` _returnvalue) Location) 1.0 false))

(fn `GetLocationUnderFinger`
  (returns (Hit :type Boolean) (Location :type "Vector Structure"))
  (bind (_bblockinghit _binitialoverlap _time _distance _location) (`GameplayStatics.BreakHitResult` (`self.GetHitResultUnderFingerByChannel` "Touch1" "TraceTypeQuery1")))
  (return _bblockinghit _location))

(fn `MoveTo`
  (params (Location :type "Vector Structure (by ref)"))
  (`AIBlueprintHelperLibrary.SimpleMoveToLocation` self Location))

(fn `UserConstructionScript`)